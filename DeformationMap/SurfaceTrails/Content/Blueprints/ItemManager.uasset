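; ItemManager spawns one item per player and summons the boss once every item is hidden and all players gather.
; While unfinished, each Tick spawns items at preset Transforms until they match the PlayerController count, then checks their hidden state.
; Afterwards, Tick spawns an AI BossCharacter high above the manager whenever none exists and every FirstPersonCharacter overlaps R.
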(event Custom|Check%20Items
  (bind _outactors (Actor|GetAllActorsOfClass "/Script/Engine.PlayerController"))
  (bind _outactors_2 (Actor|GetAllActorsOfClass "/Game/Blueprints/Item.Item_C"))
  (if (< (Utilities|Array|Length _outactors_2) (Utilities|Array|Length _outactors))
    (Game|SpawnActorfromClass "/Game/Blueprints/Item.Item_C" (Utilities|Array|Get(acopy) (Variables|Default|GetTransforms) (Utilities|Array|Length _outactors_2)) "Undefined" 0 0)
    (else
      (Variables|Default|SetNotDone false)
      (bind _array_element (Utilities|Array|ForEachLoopwithBreak _outactors_2 :!label _label)
        (:LoopBody
          (if (not (Variables|/Script/Engine.Actor|GetbHidden _array_element))
            (Variables|Default|SetNotDone true)
            (goto _label Break)))))))

(event Custom|SpawnBoss
  (AI|SpawnAIFromClass "/Game/Blueprints/BossCharacter.BossCharacter_C" 0 (+ (Transformation|GetActorLocation) "0, 0,10000.000000") "0, 0, 0" true 0))

(event EventTick
  (params (DeltaSeconds :type Float%20%28single-precision%29))
  (if (Variables|Default|GetNotDone)
    (CallFunction|CheckItems)
    (else
      (bind _outactors (Actor|GetAllActorsOfClass "/Game/FirstPersonBP/Blueprints/FirstPersonCharacter.FirstPersonCharacter_C"))
      (bind _outactors_2 (Actor|GetAllActorsOfClass "/Game/Blueprints/BossCharacter.BossCharacter_C"))
      (if (and (== (Utilities|Array|Length _outactors_2) 0) (== (Utilities|Array|Length _outactors) (Utilities|Array|Length (Collision|GetOverlappingActors (Variables|Default|Getr) "/Game/FirstPersonBP/Blueprints/FirstPersonCharacter.FirstPersonCharacter_C" :!class /Script/Engine.PrimitiveComponent))))
        (CallFunction|SpawnBoss)))))

(fn ConstructionScript)