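; BasicEnemyCharacter is an enemy that hurts the player on proximity and can catch fire, burn out and spread the flames to other enemies.
; Each tick, it drains Hp from any FirstPersonCharacter overlapping its Sphere, scaled by Damage and frame time.
; While OnFire is set, the Fire component shows and Life counts down until the actor destroys itself.
; A burning enemy ignites other BasicEnemyCharacters that begin overlapping its FireSphere.
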(event OnComponentBeginOverlap(FireSphere)
  (params (OverlappedComponent :type Primitive%20Component%20Object%20Reference) (OtherActor :type Actor%20Object%20Reference) (OtherComp :type Primitive%20Component%20Object%20Reference) (OtherBodyIndex :type Integer) (bFromSweep :type Boolean) (SweepResult :type Hit%20Result%20Structure%20%28by%20ref%29))
  (if (Variables|Default|GetOnFire)
    (bind _asbasic_enemy_character (Utilities|Casting|CastToBasicEnemyCharacter OtherActor))
    (Variables|BasicEnemyCharacter_C|SetOnFire _asbasic_enemy_character true)))

(event EventTick
  (params (DeltaSeconds :type Float%20%28single-precision%29))
  (bind _onfire (Variables|Default|GetOnFire))
  (for _array_element (Collision|GetOverlappingActors (Variables|Default|GetSphere) "/Game/FirstPersonBP/Blueprints/FirstPersonCharacter.FirstPersonCharacter_C" :!class /Script/Engine.PrimitiveComponent)
    (bind _asfirst_person_character (Utilities|Casting|CastToFirstPersonCharacter _array_element))
    (Variables|/Game/FirstPersonBP/Blueprints/FirstPersonCharacter.FirstPersonCharacter_C|SetHp _asfirst_person_character (- (Variables|/Game/FirstPersonBP/Blueprints/FirstPersonCharacter.FirstPersonCharacter_C|GetHp _asfirst_person_character) (* DeltaSeconds (Variables|Default|GetDamage)))))
  (Rendering|SetVisibility (Variables|Default|GetFire) _onfire false)
  (if _onfire
    (Variables|Default|SetLife (- (Variables|Default|GetLife) DeltaSeconds))
    (if (< (Variables|Default|GetLife) 0.0)
      (Actor|DestroyActor))))

(fn ConstructionScript)