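; BossCharacter is a boss enemy that fires projectiles at the player and ends the game when defeated.
; Each Tick it turns its Target component toward the FirstPersonCharacter and counts down a shot timer.
; When the timer drops below zero, it spawns a BossProjectile from Target's position and rotation, then resets the timer.
; Once HP falls below zero, Tick calls Win, which opens the Credits level.
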(event Custom|Shoot
  (bind _target (Variables|Default|Gettarget))
  (Game|SpawnActorfromClass "/Game/Blueprints/BossProjectile.BossProjectile_C" (Math|Transform|MakeTransform (Transformation|GetWorldLocation _target) (Transformation|GetWorldRotation _target)) "AlwaysSpawn" 0 0) ; Spawn projectile
  (Variables|Default|SetTillShoot (Variables|Default|GetBetweenShoot)))

(event Custom|Win
  (Game|OpenLevel(byName) "Credits"))

(event EventTick
  (params (DeltaSeconds :type Float%20%28single-precision%29))
  (if (< (Variables|Default|GetHP) 0.0)
    (CallFunction|Win)
    (else
      (bind _returnvalue (Actor|GetActorOfClass "/Game/FirstPersonBP/Blueprints/FirstPersonCharacter.FirstPersonCharacter_C"))
      (Variables|Default|SetLookingAt _returnvalue)
      (Transformation|SetWorldRotation (Variables|Default|Gettarget) (Math|Rotator|FindLookatRotation (Transformation|GetWorldLocation (Variables|Default|Gettarget)) (Transformation|GetActorLocation (Variables|Default|GetLookingAt))) false false)
      (Variables|Default|SetTillShoot (- (Variables|Default|GetTillShoot) DeltaSeconds))
      (if (< (Variables|Default|GetTillShoot) 0.0)
        (CallFunction|Shoot)))))

(fn ConstructionScript)