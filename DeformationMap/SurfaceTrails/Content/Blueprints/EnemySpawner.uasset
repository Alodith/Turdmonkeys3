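; Enemy spawner actor that periodically spawns a BasicEnemyCharacter AI just above its own location.
; Tick counts TillSpawn down, then requires the world's enemy count to be under a cap and a FirstPersonCharacter to pass a distance check.
; That check joins its near and far limits with OR, so any existing player character passes.
; SpawnEnemy resets the timer to SpawnInterval, so blocked attempts retry every tick.
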(event Custom|SpawnEnemy
  (AI|SpawnAIFromClass "/Game/Blueprints/BasicEnemyCharacter.BasicEnemyCharacter_C" 0 (+ (Transformation|GetActorLocation) "0, 0,100.000000") "0, 0, 0" true 0)
  (Variables|Default|SetTillSpawn (Variables|Default|GetSpawnInterval)))

(event EventTick
  (params (DeltaSeconds :type Float%20%28single-precision%29))
  (Variables|Default|SetTillSpawn (- (Variables|Default|GetTillSpawn) DeltaSeconds))
  (if (< (Variables|Default|GetTillSpawn) 0.0)
    (bind _outactors (Actor|GetAllActorsOfClass "/Game/Blueprints/BasicEnemyCharacter.BasicEnemyCharacter_C"))
    (if (< (Utilities|Array|Length _outactors) 100)
      (Variables|Default|SetCanSpawn false)
      (bind _outactors_2 (Actor|GetAllActorsOfClass "/Game/FirstPersonBP/Blueprints/FirstPersonCharacter.FirstPersonCharacter_C"))
      (bind _array_element (Utilities|Array|ForEachLoopwithBreak _outactors_2 :!label _label)
        (:LoopBody
          (if (or (< (Math|Vector|Distance(Vector) (Transformation|GetActorLocation _array_element) (Transformation|GetActorLocation)) 1e+04) (> (Math|Vector|Distance(Vector) (Transformation|GetActorLocation _array_element) (Transformation|GetActorLocation)) 2.5e+03))
            (Variables|Default|SetCanSpawn true)
            (goto _label Break)))
        (:Completed
          (if (Variables|Default|GetCanSpawn)
            (CallFunction|SpawnEnemy)))))))

(fn ConstructionScript)