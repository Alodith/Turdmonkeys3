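; AI controller for a basic enemy that chases the nearest player.
; On possess, it scans all PlayerController actors, starting from player 0, and keeps the closest by distance as Target.
; Tick issues MoveToActor toward that Target, re-running the search only when it becomes invalid.
; Distance checks and movement use the PlayerController actors themselves, rather than their pawns.
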(event Custom|GetTarget
  (bind _outactors (Actor|GetAllActorsOfClass "/Script/Engine.PlayerController"))
  (Variables|Default|SetPlayers _outactors)
  (Variables|Default|SetTarget (Game|GetPlayerController 0))
  (for _array_element (Variables|Default|GetPlayers)
    (if (< (Transformation|GetDistanceTo _array_element) (Transformation|GetDistanceTo (Variables|Default|GetTarget)))
      (Variables|Default|SetTarget _array_element))))

(event EventTick
  (params (DeltaSeconds :type Float%20%28single-precision%29))
  (if (Utilities|IsValid (Variables|Default|GetTarget))
    (AI|Navigation|MovetoActor (Variables|Default|GetTarget) -1.0 true true true 0)
    (else
      (CallFunction|GetTarget))))

(event EventPossess
  (params (PossessedPawn :type Pawn%20Object%20Reference))
  (CallFunction|GetTarget))

(fn ConstructionScript)