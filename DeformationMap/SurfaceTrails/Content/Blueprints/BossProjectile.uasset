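; BossProjectile is a projectile actor that moves forward at a fixed speed and drains the first-person character's health on contact.
; Each tick it sweeps along its forward vector, then reduces Hp on every overlapping FirstPersonCharacter, scaled by delta time.
; On beginning overlap with an actor of exactly the BasicEnemyCharacter class, it clears that enemy's OnFire flag.
; The graph contains no logic to destroy the projectile.
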(event Collision|EventActorBeginOverlap
  (params (OtherActor :type Actor%20Object%20Reference))
  (if (== (Utilities|GetClass OtherActor) "/Game/Blueprints/BasicEnemyCharacter.BasicEnemyCharacter_C")
    (bind _asbasic_enemy_character (Utilities|Casting|CastToBasicEnemyCharacter OtherActor))
    (Variables|/Game/Blueprints/BasicEnemyCharacter.BasicEnemyCharacter_C|SetOnFire _asbasic_enemy_character false)))

(event EventTick
  (params (DeltaSeconds :type Float%20%28single-precision%29))
  (Transformation|SetActorLocation (+ (Transformation|GetActorLocation) (* (* (Math|Vector|GetForwardVector (Transformation|GetActorRotation)) DeltaSeconds) 2e+03)) true false)
  (for _array_element (Collision|GetOverlappingActors "/Game/FirstPersonBP/Blueprints/FirstPersonCharacter.FirstPersonCharacter_C" :!class /Script/Engine.Actor)
    (bind _asfirst_person_character (Utilities|Casting|CastToFirstPersonCharacter _array_element))
    (Variables|/Game/FirstPersonBP/Blueprints/FirstPersonCharacter.FirstPersonCharacter_C|SetHp _asfirst_person_character (- (Variables|/Game/FirstPersonBP/Blueprints/FirstPersonCharacter.FirstPersonCharacter_C|GetHp _asfirst_person_character) (* DeltaSeconds 5.0)))))

(fn ConstructionScript)